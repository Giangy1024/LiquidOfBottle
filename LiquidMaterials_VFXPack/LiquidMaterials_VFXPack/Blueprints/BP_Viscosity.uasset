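; BP_Viscosity is a demo actor in the liquid materials pack that moves three bottles in unison along the world X axis, apparently to showcase viscosity.
; BeginPlay caches each bottle's starting world location, then plays the Movements timeline from the start.
; Each update offsets the bottles from those origins by the Movement3 track value, re-centred around 0.5 and scaled into a horizontal distance, without sweeping.
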(event EventBeginPlay
  (Variables|Default|SetBottle1_Loc (Transformation|GetWorldLocation (Variables|Default|GetBottle01)))
  (Variables|Default|SetBottle2_Loc (Transformation|GetWorldLocation (Variables|Default|GetBottle02)))
  (Variables|Default|SetBottle3_Loc (Transformation|GetWorldLocation (Variables|Default|GetBottle03)))
  (bind _movement3 (Timeline|Movements PlayFromStart)
    (:Update
      (Transformation|SetWorldLocation (Variables|Default|GetBottle01) (+ (* (- _movement3 0.5) "400.000000,0.000000,0.000000") (Variables|Default|GetBottle1_Loc)) false false)
      (Transformation|SetWorldLocation (Variables|Default|GetBottle02) (+ (* (- _movement3 0.5) "400.000000,0.000000,0.000000") (Variables|Default|GetBottle2_Loc)) false false)
      (Transformation|SetWorldLocation (Variables|Default|GetBottle03) (+ (* (- _movement3 0.5) "400.000000,0.000000,0.000000") (Variables|Default|GetBottle3_Loc)) false false))))

(event Collision|EventActorBeginOverlap
  (params (OtherActor :type Actor%20Object%20Reference)))

(event EventTick
  (params (DeltaSeconds :type Float%20%28single-precision%29)))

(fn ConstructionScript)