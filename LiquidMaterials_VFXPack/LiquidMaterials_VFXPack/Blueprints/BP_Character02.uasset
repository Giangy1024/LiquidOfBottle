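; Demo character that moves by itself along a circular path, alternating between timed walking and pausing phases.
; Tick ramps Speed up or down with the Stop flag and uses it for both yaw rotation and forward offset.
; Paired DoOnce nodes and Delays toggle Stop and mirror it to AnimBP_Character.
; The construction script sets a FadeDistance material parameter on StaticMesh1.
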(event EventBeginPlay
  (bind _asanim_bp_character (Utilities|Casting|CastToAnimBP_Character (Components|SkeletalMesh|GetAnimInstance (Variables|Character|GetMesh))))
  (Variables|Default|SetAnimBP _asanim_bp_character))

(event EventTick
  (params (DeltaSeconds :type Float%20%28single-precision%29))
  (Utilities|FlowControl|Sequence
    (:then_0
      (if (Variables|Default|Getstop)
        (Variables|Default|SetSpeed (Math|Float|Max(Float) (- (Variables|Default|GetSpeed) 4.0) 0.0))
        (Utilities|FlowControl|DoOnce false :!label _label
          (:Completed
            (Variables|/Game/LiquidMaterials_VFXPack/Demo/Character/AnimBP_Character.AnimBP_Character_C|SetStop (Variables|Default|GetAnimBP) true)
            (Utilities|FlowControl|Sequence
              (:then_0
                (Utilities|FlowControl|Delay 3.0)
                (Variables|Default|Setstop false))
              (:then_1
                (goto _label_2 Reset)))))
        (else
          (Utilities|FlowControl|Sequence
            (:then_0
              (Variables|Default|SetSpeed (Math|Float|Min(Float) (+ (Variables|Default|GetSpeed) 4.0) 6e+01))
              (Utilities|FlowControl|DoOnce false :!label _label_2
                (:Completed
                  (Variables|/Game/LiquidMaterials_VFXPack/Demo/Character/AnimBP_Character.AnimBP_Character_C|SetStop (Variables|Default|GetAnimBP) false)
                  (Utilities|FlowControl|Sequence
                    (:then_0
                      (Utilities|FlowControl|Delay 5.0)
                      (Variables|Default|Setstop true))
                    (:then_1
                      (goto _label Reset))))))))))
    (:then_1
      (Class|Actor|AddActorWorldRotation (Math|Rotator|MakeRotator 0.0 0.0 (* DeltaSeconds (Variables|Default|GetSpeed))))
      (Transformation|AddActorLocalOffset (Math|Vector|MakeVector (* (* DeltaSeconds (Variables|Default|GetSpeed)) 8.0) 0.0 0.0) false false))))

(fn ConstructionScript
  (Rendering|Material|SetScalarParameterValueonMaterials (Variables|Default|GetStaticMesh1) "FadeDistance" 2.5e+02))