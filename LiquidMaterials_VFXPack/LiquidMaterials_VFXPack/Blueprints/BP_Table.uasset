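; Demo table for the liquid VFX pack that repeatedly tilts thirteen physics-simulated bottles and replaces them.
; The construction script spawns glass bottles from a struct array, each with an attached stopper and Niagara liquid using that entry's mesh and size, plus random material and fill.
; From BeginPlay, a delayed Timeline rolls the Cube.
; When it finishes, all bottles are destroyed and respawned with random bottle materials, and the cycle restarts.
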(event Custom|Again
  (bind _cube (Variables|Default|GetCube))
  (bind _returnvalue (Transformation|GetWorldTransform _cube))
  (Utilities|FlowControl|Delay 4.0)
  (bind _newtrack_0 (Timeline|Timeline PlayFromStart)
    (:Update
      (Transformation|SetWorldRotation (Variables|Default|GetCube) (Math|Rotator|MakeRotator (* _newtrack_0 45.0) 0.0 0.0) false false))
    (:Finished
      (for _array_element (Variables|Default|GetBottle)
        (if (Utilities|IsValid _array_element)
          (Components|DestroyComponent _array_element)))
      (for _array_element_2 (Variables|Default|GetNiagaraSys)
        (if (Utilities|IsValid _array_element_2)
          (Components|DestroyComponent _array_element_2)))
      (for _array_element_3 (Variables|Default|GetStopper)
        (if (Utilities|IsValid _array_element_3)
          (Components|DestroyComponent _array_element_3)))
      (Utilities|Array|Clear (Variables|Default|GetBottle))
      (Utilities|Array|Clear (Variables|Default|GetNiagaraSys))
      (Utilities|Array|Clear (Variables|Default|GetStopper))
      (Variables|Default|SetBottles 0)
      (while (< (Variables|Default|GetBottles) 13)
        (Variables|Default|SetRandomV (Variables|Default|GetBottles))
        (bind _returnvalue_2 (AddComponent|AddStaticMeshComponent true (Math|Transform|MakeTransform (+ (.location _returnvalue) (Math|Vector|MakeVector (- (+ (Math|Random|RandomFloatinRange -1e+01 1e+01) (* (Variables|Default|GetBottles) 35.0)) 2e+02) (Math|Random|RandomFloatinRange -2e+01 2e+01) 2e+01)) (Math|Rotator|MakeRotator (.roll (.rotation _returnvalue)) (.pitch (.rotation _returnvalue)) (Math|Random|RandomFloatinRange 0.0 3.6e+02)) (Math|Vector|MakeVector 1.0 1.0 1.0))))
        (Utilities|Array|AddUnique (Variables|Default|GetBottle) _returnvalue_2)
        (Physics|SetSimulatePhysics _returnvalue_2 true)
        (Components|StaticMesh|SetStaticMesh _returnvalue_2 (.bottle (Utilities|Array|Get(acopy) (Variables|Default|GetStructure_Bottles) (Variables|Default|GetRandomV))))
        (Rendering|Material|SetMaterial _returnvalue_2 0 (.OutItem (Utilities|Array|Random (Variables|Default|GetMaterialBottle))))
        (bind _returnvalue_3 (AddComponent|AddNiagaraComponent true))
        (Utilities|Array|AddUnique (Variables|Default|GetNiagaraSys) _returnvalue_3)
        (Class|NiagaraComponent|SetAsset _returnvalue_3 "/Game/LiquidMaterials_VFXPack/Effects/P_Liquid.P_Liquid" true)
        (Transformation|AttachComponentToComponent _returnvalue_3 _returnvalue_2 "None" "SnapToTarget" "SnapToTarget" "SnapToTarget" true)
        (Class|NiagaraComponent|SetVariableStaticMesh _returnvalue_3 "User.Mesh" (.liquid (Utilities|Array|Get(acopy) (Variables|Default|GetStructure_Bottles) (Variables|Default|GetRandomV))))
        (Class|NiagaraComponent|SetVariableMaterial _returnvalue_3 "User.Material" (.OutItem (Utilities|Array|Random (Variables|Default|GetObject))))
        (Effects|Components|ParticleSystem|SetVectorParameter _returnvalue_3 "User.BottleSize" (.bottlesize (Utilities|Array|Get(acopy) (Variables|Default|GetStructure_Bottles) (Variables|Default|GetRandomV))))
        (Effects|Components|ParticleSystem|SetFloatParameter _returnvalue_3 "User.Fill" (Math|Random|RandomFloatinRange 0.25 0.85))
        (bind _returnvalue_4 (AddComponent|AddStaticMeshComponent false))
        (Utilities|Array|AddUnique (Variables|Default|GetStopper) _returnvalue_4)
        (Components|StaticMesh|SetStaticMesh _returnvalue_4 (.stopper (Utilities|Array|Get(acopy) (Variables|Default|GetStructure_Bottles) (Variables|Default|GetRandomV))))
        (Transformation|AttachComponentToComponent _returnvalue_4 _returnvalue_2 "None" "SnapToTarget" "SnapToTarget" "SnapToTarget" true)
        (Math|Integer|IncrementInt (Variables|Default|GetBottles)))
      (CallFunction|Again))))

(event EventBeginPlay
  (bind _cube (Variables|Default|GetCube))
  (bind _returnvalue (Transformation|GetWorldTransform _cube))
  (Utilities|FlowControl|Delay 4.0)
  (bind _newtrack_0 (Timeline|Timeline PlayFromStart)
    (:Update
      (Transformation|SetWorldRotation (Variables|Default|GetCube) (Math|Rotator|MakeRotator (* _newtrack_0 45.0) 0.0 0.0) false false))
    (:Finished
      (for _array_element (Variables|Default|GetBottle)
        (if (Utilities|IsValid _array_element)
          (Components|DestroyComponent _array_element)))
      (for _array_element_2 (Variables|Default|GetNiagaraSys)
        (if (Utilities|IsValid _array_element_2)
          (Components|DestroyComponent _array_element_2)))
      (for _array_element_3 (Variables|Default|GetStopper)
        (if (Utilities|IsValid _array_element_3)
          (Components|DestroyComponent _array_element_3)))
      (Utilities|Array|Clear (Variables|Default|GetBottle))
      (Utilities|Array|Clear (Variables|Default|GetNiagaraSys))
      (Utilities|Array|Clear (Variables|Default|GetStopper))
      (Variables|Default|SetBottles 0)
      (while (< (Variables|Default|GetBottles) 13)
        (Variables|Default|SetRandomV (Variables|Default|GetBottles))
        (bind _returnvalue_2 (AddComponent|AddStaticMeshComponent true (Math|Transform|MakeTransform (+ (.location _returnvalue) (Math|Vector|MakeVector (- (+ (Math|Random|RandomFloatinRange -1e+01 1e+01) (* (Variables|Default|GetBottles) 35.0)) 2e+02) (Math|Random|RandomFloatinRange -2e+01 2e+01) 2e+01)) (Math|Rotator|MakeRotator (.roll (.rotation _returnvalue)) (.pitch (.rotation _returnvalue)) (Math|Random|RandomFloatinRange 0.0 3.6e+02)) (Math|Vector|MakeVector 1.0 1.0 1.0))))
        (Utilities|Array|AddUnique (Variables|Default|GetBottle) _returnvalue_2)
        (Physics|SetSimulatePhysics _returnvalue_2 true)
        (Components|StaticMesh|SetStaticMesh _returnvalue_2 (.bottle (Utilities|Array|Get(acopy) (Variables|Default|GetStructure_Bottles) (Variables|Default|GetRandomV))))
        (Rendering|Material|SetMaterial _returnvalue_2 0 (.OutItem (Utilities|Array|Random (Variables|Default|GetMaterialBottle))))
        (bind _returnvalue_3 (AddComponent|AddNiagaraComponent true))
        (Utilities|Array|AddUnique (Variables|Default|GetNiagaraSys) _returnvalue_3)
        (Class|NiagaraComponent|SetAsset _returnvalue_3 "/Game/LiquidMaterials_VFXPack/Effects/P_Liquid.P_Liquid" true)
        (Transformation|AttachComponentToComponent _returnvalue_3 _returnvalue_2 "None" "SnapToTarget" "SnapToTarget" "SnapToTarget" true)
        (Class|NiagaraComponent|SetVariableStaticMesh _returnvalue_3 "User.Mesh" (.liquid (Utilities|Array|Get(acopy) (Variables|Default|GetStructure_Bottles) (Variables|Default|GetRandomV))))
        (Class|NiagaraComponent|SetVariableMaterial _returnvalue_3 "User.Material" (.OutItem (Utilities|Array|Random (Variables|Default|GetObject))))
        (Effects|Components|ParticleSystem|SetVectorParameter _returnvalue_3 "User.BottleSize" (.bottlesize (Utilities|Array|Get(acopy) (Variables|Default|GetStructure_Bottles) (Variables|Default|GetRandomV))))
        (Effects|Components|ParticleSystem|SetFloatParameter _returnvalue_3 "User.Fill" (Math|Random|RandomFloatinRange 0.25 0.85))
        (bind _returnvalue_4 (AddComponent|AddStaticMeshComponent false))
        (Utilities|Array|AddUnique (Variables|Default|GetStopper) _returnvalue_4)
        (Components|StaticMesh|SetStaticMesh _returnvalue_4 (.stopper (Utilities|Array|Get(acopy) (Variables|Default|GetStructure_Bottles) (Variables|Default|GetRandomV))))
        (Transformation|AttachComponentToComponent _returnvalue_4 _returnvalue_2 "None" "SnapToTarget" "SnapToTarget" "SnapToTarget" true)
        (Math|Integer|IncrementInt (Variables|Default|GetBottles)))
      (CallFunction|Again))))

(fn ConstructionScript
  (bind _cube (Variables|Default|GetCube))
  (bind _returnvalue (Transformation|GetWorldTransform _cube))
  (Utilities|Array|Clear (Variables|Default|GetBottle))
  (Utilities|Array|Clear (Variables|Default|GetNiagaraSys))
  (Utilities|Array|Clear (Variables|Default|GetStopper))
  (Variables|Default|SetBottles 0)
  (while (< (Variables|Default|GetBottles) 13)
    (Variables|Default|SetRandomV (Variables|Default|GetBottles))
    (bind _returnvalue_2 (AddComponent|AddStaticMeshComponent true (Math|Transform|MakeTransform (+ (.location _returnvalue) (Math|Vector|MakeVector (- (+ (Math|Random|RandomFloatinRange -1e+01 1e+01) (* (Variables|Default|GetBottles) 35.0)) 2e+02) (Math|Random|RandomFloatinRange -2e+01 2e+01) 2e+01)) (Math|Rotator|MakeRotator (.roll (.rotation _returnvalue)) (.pitch (.rotation _returnvalue)) (Math|Random|RandomFloatinRange 0.0 3.6e+02)) (Math|Vector|MakeVector 1.0 1.0 1.0))))
    (Utilities|Array|AddUnique (Variables|Default|GetBottle) _returnvalue_2)
    (Physics|SetSimulatePhysics _returnvalue_2 true)
    (Components|StaticMesh|SetStaticMesh _returnvalue_2 (.bottle (Utilities|Array|Get(acopy) (Variables|Default|GetStructure_Bottles) (Variables|Default|GetRandomV))))
    (Rendering|Material|SetMaterial _returnvalue_2 0 "/Game/LiquidMaterials_VFXPack/Materials/M_Glass.M_Glass")
    (bind _returnvalue_3 (AddComponent|AddNiagaraComponent true))
    (Utilities|Array|AddUnique (Variables|Default|GetNiagaraSys) _returnvalue_3)
    (Class|NiagaraComponent|SetAsset _returnvalue_3 "/Game/LiquidMaterials_VFXPack/Effects/P_Liquid.P_Liquid" true)
    (Transformation|AttachComponentToComponent _returnvalue_3 _returnvalue_2 "None" "SnapToTarget" "SnapToTarget" "SnapToTarget" true)
    (Class|NiagaraComponent|SetVariableStaticMesh _returnvalue_3 "User.Mesh" (.liquid (Utilities|Array|Get(acopy) (Variables|Default|GetStructure_Bottles) (Variables|Default|GetRandomV))))
    (Class|NiagaraComponent|SetVariableMaterial _returnvalue_3 "User.Material" (.OutItem (Utilities|Array|Random (Variables|Default|GetObject))))
    (Effects|Components|ParticleSystem|SetVectorParameter _returnvalue_3 "User.BottleSize" (.bottlesize (Utilities|Array|Get(acopy) (Variables|Default|GetStructure_Bottles) (Variables|Default|GetRandomV))))
    (Effects|Components|ParticleSystem|SetFloatParameter _returnvalue_3 "User.Fill" (Math|Random|RandomFloatinRange 0.25 0.85))
    (bind _returnvalue_4 (AddComponent|AddStaticMeshComponent false))
    (Utilities|Array|AddUnique (Variables|Default|GetStopper) _returnvalue_4)
    (Components|StaticMesh|SetStaticMesh _returnvalue_4 (.stopper (Utilities|Array|Get(acopy) (Variables|Default|GetStructure_Bottles) (Variables|Default|GetRandomV))))
    (Transformation|AttachComponentToComponent _returnvalue_4 _returnvalue_2 "None" "SnapToTarget" "SnapToTarget" "SnapToTarget" true)
    (Math|Integer|IncrementInt (Variables|Default|GetBottles))))